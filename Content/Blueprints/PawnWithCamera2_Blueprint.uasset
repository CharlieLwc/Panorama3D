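; A camera pawn Blueprint that feeds the VR viewer's camera position to a material.
; Each Tick it writes the player camera manager's location into the VRCamPos vector parameter of the RVMatInst material instance.
; It also prints that location and the headset's device position as debug output.
; BeginPlay, overlap and construction script are empty, and the OurCamera transform nodes are left unconnected.
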(event EventBeginPlay)

(event EventActorBeginOverlap
  (params (OtherActor :type Actor%20Object%20Reference)))

(event EventTick
  (params (DeltaSeconds :type Float%20%28single-precision%29))
  (bind _returnvalue (Game|GetPlayerCameraManager 0))
  (bind _returnvalue_2 (Camera|GetCameraLocation _returnvalue))
  (Rendering|Material|SetVectorParameterValue (Variables|Default|GetRV_MatInst) "VRCamPos" (Math|Conversions|ToLinearColor(Vector) _returnvalue_2) :!class /Script/Engine.MaterialInstanceDynamic)
  (Development|PrintString (Utilities|String|ToString(Vector) _returnvalue_2))
  (Development|PrintString (Utilities|String|ToString(Vector) (.DevicePosition (Class|HeadMountedDisplayFunctionLibrary|GetOrientationandPosition)))))

(fn ConstructionScript)